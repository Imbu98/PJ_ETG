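; Damage component that tracks its owner's HP and sends a die message to the owner when HP runs out.
; A state check gates incoming damage, blocking it while invincible, or while dodging if the hit is dodgeable.
; Surviving hits make player-team owners temporarily invincible and tint dynamic instances of the first two skeletal mesh materials red.
; After a short delay the tint clears and the state returns to Idle.
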(event Custom|ComponentDamaged
  (params (Amount :type Float%20%28double-precision%29) (CanDodge :type Boolean))
  (bind _returnvalue (Components|GetOwner))
  (Utilities|StateJudgement (Variables|Default|GetCurrentState) CanDodge
    (:DoDamage
      (bind _output_get (Variables|Default|SetCurrentHp (- (Variables|Default|GetCurrentHp) Amount)))
      (if (<= _output_get 0.0)
        (Utilities|IsValid _returnvalue
          (:Is%20Valid
            (Class|BPIDamage|SetStateDie(Message) _returnvalue)))
        (else
          ;[0.15 0.15 0.15 0.5] 플레이어만 무적처리
          (bind _teamdefinition (Class|BPIDamage|GetTeam(Message) _returnvalue))
          (if (Utilities|Enum|Equal(Enum) _teamdefinition "NewEnumerator0")
            (Variables|Default|SetCurrentState "NewEnumerator1"))
          ;[0.15 0.15 0.15 0.5] 피격시 머테리얼 변경
          (Utilities|FlowControl|Sequence
            (:then_0
              (for _array_element (Variables|Default|GetMaterialInstance1)
                (Rendering|Material|SetVectorParameterValue _array_element "Tint" "(R=1.000000,G=0.000000,B=0.003297,A=1.000000)" :!class /Script/Engine.MaterialInstanceDynamic))
              (Utilities|FlowControl|Delay 0.5)
              (for _array_element_2 (Variables|Default|GetMaterialInstance1)
                (Rendering|Material|SetVectorParameterValue _array_element_2 "Tint" "(R=1.000000,G=1.000000,B=1.000000,A=1.000000)" :!class /Script/Engine.MaterialInstanceDynamic))
              (Variables|Default|SetCurrentState "NewEnumerator0"))))))))

(event EventBeginPlay
  (bind _returnvalue (Components|GetOwner))
  (bind _materialinstance1 (Variables|Default|GetMaterialInstance1))
  (bind _returnvalue_2 (Actor|GetComponentbyClass _returnvalue "/Script/Engine.SkeletalMeshComponent"))
  (Variables|Default|SetCurrentHp (Variables|Default|GetMaxHp))
  (Utilities|IsValid _returnvalue_2
    (:Is%20Valid
      (bind _returnvalue_3 (Rendering|Material|CreateDynamicMaterialInstance _returnvalue_2 0 (Rendering|Material|GetMaterial _returnvalue_2 0) "None" :!class /Script/Engine.PrimitiveComponent))
      (bind _returnvalue_4 (Rendering|Material|CreateDynamicMaterialInstance _returnvalue_2 1 (Rendering|Material|GetMaterial _returnvalue_2 1) "None" :!class /Script/Engine.PrimitiveComponent))
      (Utilities|Array|Add _materialinstance1 _returnvalue_4)
      (Utilities|Array|Add _materialinstance1 _returnvalue_3))))

(event EventTick
  (params (DeltaSeconds :type Float%20%28single-precision%29)))