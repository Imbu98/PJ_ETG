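; BP_Chest is an interactable loot chest that spawns a weapon pickup based on its rarity.
; On Interact, GetRowName maps ChestRarity to a row in GunDataTable, which holds that tier's Weapons array.
; A random index expression selects the entry, evaluated separately for the non-zero ItemID check and for the spawn.
; A successful roll spawns an enlarged BP_HT_WeaponPickUpBase above the chest and disables further interaction.
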(event EventInteract
  (params (Player :type Actor%20Object%20Reference))
  (if (Variables|Default|GetbCanInteract)
    (bind _returnvalue (Utilities|GetDataTableRow (Variables|Default|GetGunDataTable) (CallFunction|GetRowName))
      (:then
        (if (!= (.ItemID (Utilities|Struct|BreakS_WeaponCompoent (Utilities|Array|Get(acopy) (Utilities|Struct|BreakS_WeaponComponentArray _returnvalue) (Math|Random|RandomIntegerinRange 0 (- 1 (Utilities|Array|Length (Utilities|Struct|BreakS_WeaponComponentArray _returnvalue))))))) 0)
          (Game|SpawnActorfromClass "/Game/HyoTaek/Blueprints/GunInteractBase/BP_HT_WeaponPickUpBase.BP_HT_WeaponPickUpBase_C" (Math|Transform|MakeTransform (+ (Transformation|GetActorLocation) "0.000000,0.000000,150.000000") "0, 0, 0" "2.000000,2.000000,2.000000") "AlwaysSpawn" "MultiplyWithRoot" 0 (Utilities|Array|Get(acopy) (Utilities|Struct|BreakS_WeaponComponentArray _returnvalue) (Math|Random|RandomIntegerinRange 0 (- 1 (Utilities|Array|Length (Utilities|Struct|BreakS_WeaponComponentArray _returnvalue))))) 0)
          (Variables|Default|SetbCanInteract false))))))

(fn ConstructionScript
  (|CallParentFunction))

(fn GetRowName
  (switch Utilities|FlowControl|Switch|SwitchonE_Rarity (Variables|Default|GetChestRarity)
    (:NewEnumerator0
      (return (Utilities|Name|MakeLiteralName "Normal")))
    (:NewEnumerator1
      (return (Utilities|Name|MakeLiteralName "Rare")))
    (:NewEnumerator2
      (return (Utilities|Name|MakeLiteralName "Epic")))
    (:NewEnumerator3
      (return (Utilities|Name|MakeLiteralName "Legendary")))))