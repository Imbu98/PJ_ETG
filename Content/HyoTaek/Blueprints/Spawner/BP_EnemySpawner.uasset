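; Enemy spawner that creates a set of BP_HT_Robot at BeginPlay, tracks them in an array and gives each a back-reference.
; SpawnChest totals probability × weight from a data table, then spawns a BP_Chest at the spawner with a rolled rarity and matching material.
; SetChestProbability walks DT_ChestProbability cumulatively, re-rolling the random value on each row.
; An older hard-coded rarity chain remains unconnected.
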(event EventBeginPlay
  (for _index (range 0 (Variables|Default|GetSpawnActorAmount))
    (bind _returnvalue (Game|SpawnActorfromClass "/Game/HyoTaek/Character/Enemy/BP_HT_Robot.BP_HT_Robot_C" (Math|Transform|MakeTransform "0, 0, 0" "0, 0, 0" "1.000000,1.000000,1.000000") "Undefined" "MultiplyWithRoot" 0 0))
    (Utilities|Array|Add (Variables|Default|GetEnemyArray) _returnvalue)
    (Variables|/Game/HyoTaek/Character/Enemy/BP_HT_EnemyChar.BP_HT_EnemyChar_C|SetSpawner _returnvalue self)))

(fn ConstructionScript)

(fn SetChestProbability
  (params (ChestProbability :type Float%20%28double-precision%29))
  (bind _outrownames (DataTable|GetDataTableRowNames "/Game/HyoTaek/Data/DataTable/DT_ChestProbability.DT_ChestProbability"))
  (for (_array_element _array_index) _outrownames
    (bind _returnvalue (Utilities|GetDataTableRow "/Game/HyoTaek/Data/DataTable/DT_ChestProbability.DT_ChestProbability" _array_element)
      (:then
        (bind _output_get (LocalVariables|SetAcc (+ (LocalVariables|GetAcc) (* (.probability _returnvalue) (.weight _returnvalue)))))
        (if (<= (Math|Random|RandomFloatinRange 0.0 ChestProbability) _output_get)
          (return (Utilities|Enum|ByteToEnumE_Rarity (Math|Conversions|ToByte(Integer) _array_index))))))))

(fn SpawnChest
  (bind _output_get (Variables|Default|SetProbabilityDataTable (.DataTable (Utilities|Struct|BreakDataTableRowHandle (Variables|Default|GetDT_ChestProbability)))))
  (Utilities|IsValid _output_get
    (:Is%20Valid
      (Utilities|FlowControl|Sequence
        (:then_0
          (bind _outrownames (DataTable|GetDataTableRowNames (Variables|Default|GetProbabilityDataTable)))
          (for _array_element _outrownames
            (bind _returnvalue (Utilities|GetDataTableRow (Variables|Default|GetProbabilityDataTable) _array_element)
              (:then
                (bind _output_get_2 (Variables|Default|SetTotalProbability (+ (Variables|Default|GetTotalProbability) (* (.Probability (Utilities|Struct|BreakS_ChestProbability _returnvalue)) (.Weight (Utilities|Struct|BreakS_ChestProbability _returnvalue)))))))))
          (bind _rarity (CallFunction|SetChestProbability _output_get_2))
          (Variables|Default|SetTotalProbability 0.0))
        (:then_1
          (bind _returnvalue_2 (Game|SpawnActorfromClass "/Game/HyoTaek/Blueprints/Chest/BP_Chest.BP_Chest_C" (Math|Transform|MakeTransform (Transformation|GetActorLocation) "0, 0, 0" "1.000000,1.000000,1.000000") "Undefined" "MultiplyWithRoot" 0 _rarity 0))
          (Utilities|IsValid _returnvalue_2
            (:Is%20Valid
              (bind _returnvalue_3 (Utilities|GetDataTableRow "/Game/HyoTaek/Data/DataTable/DT_ChestComponent.DT_ChestComponent" (Utilities|Select :Index _rarity :NewEnumerator0 "Normal" :NewEnumerator1 "Rare" :NewEnumerator2 "Epic" :NewEnumerator3 "Legendary"))
                (:then
                  (Rendering|Material|SetMaterial (Variables|/Game/HyoTaek/Blueprints/Chest/BP_Chest.BP_Chest_C|GetStaticMesh _returnvalue_2) 0 (.chestmaterial _returnvalue_3)))))))))))