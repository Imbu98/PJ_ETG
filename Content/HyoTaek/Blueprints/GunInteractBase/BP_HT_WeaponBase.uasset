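; Base weapon actor whose visible mesh is supplied by its current weapon component.
; On BeginPlay it calls the parent, then applies the component's GunMesh to the Cube static mesh component if that mesh is valid.
; Overlap and Tick events are disabled, and the construction script only calls its parent.
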(event EventBeginPlay
  (bind _currentweaponcomponent (Variables|Default|GetCurrentWeaponComponent))
  (|CallParentFunction)
  (Utilities|IsValid (.gunmesh _currentweaponcomponent)
    (:Is%20Valid
      (Components|StaticMesh|SetStaticMesh (Variables|Default|GetCube) (.gunmesh _currentweaponcomponent)))))

(event Collision|EventActorBeginOverlap
  (params (OtherActor :type Actor%20Object%20Reference))
  (|CallParentFunction OtherActor) ; This node is disabled and will not be called.\nDrag off pins to build functionality.
)

(event EventTick
  (params (DeltaSeconds :type Float%20%28single-precision%29))
  (|CallParentFunction DeltaSeconds) ; This node is disabled and will not be called.\nDrag off pins to build functionality.
)

(fn ConstructionScript
  (|CallParentFunction))