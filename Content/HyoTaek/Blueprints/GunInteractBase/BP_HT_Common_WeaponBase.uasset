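; Common weapon base actor that provides two fire functions, both spawning projectiles at its Muzzle.
; PistolFire spawns a BP_HT_Bullet, while RifleFire, despite its name, throws a BP_JS_Bomb toward the point under the cursor.
; The throw solves ballistic launch speed from horizontal distance, BombDegree and the owning Character's gravity, ignoring muzzle height.
; It passes the resulting horizontal and vertical velocity vectors to the bomb.
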(event EventBeginPlay
  (|CallParentFunction))

(event Collision|EventActorBeginOverlap
  (params (OtherActor :type Actor%20Object%20Reference))
  (|CallParentFunction OtherActor) ; This node is disabled and will not be called.\nDrag off pins to build functionality.
)

(event EventTick
  (params (DeltaSeconds :type Float%20%28single-precision%29))
  (|CallParentFunction DeltaSeconds) ; This node is disabled and will not be called.\nDrag off pins to build functionality.
)

(fn ConstructionScript
  (|CallParentFunction))

(fn PistolFire
  (Game|SpawnActorfromClass "/Game/HyoTaek/Blueprints/Bullet/BP_HT_Bullet.BP_HT_Bullet_C" (Transformation|GetWorldTransform (Variables|Default|GetMuzzle)) "Undefined" "MultiplyWithRoot" 0 "NewEnumerator0" 0))

(fn RifleFire
  (bind _bombdegree (Variables|Default|GetBombDegree))
  (bind _bombdegree_2 (Variables|Default|GetBombDegree))
  (bind _muzzle (Variables|Default|GetMuzzle))
  (bind _returnvalue (Transformation|GetWorldLocation _muzzle))
  (bind _returnvalue_2 (Math|Trig|Cos(Degrees) _bombdegree))
  ;[0.15 0.15 0.15 0.5] 폭탄던지기
  ;;[0.15 0.15 0.15 0.5] 클릭한 지점 위치
  (bind _output_get (Variables|Default|SetClick%20Location (.Location (Collision|BreakHitResult (.HitResult (Game|Player|GetHitResultUnderCursorbyChannel (Game|GetPlayerController 0) "TraceTypeQuery1" true))))))
  (bind _output_get_2 (Variables|Default|SetR (Math|Float|Sqrt (+ (Math|Float|Power (- (.x _output_get) (.x _returnvalue)) 2.0) (Math|Float|Power (- (.y _output_get) (.y _returnvalue)) 2.0))))) ; 시작과 도착 사이의 수평거리
  (bind _ascharacter (Utilities|Casting|CastToCharacter (Components|GetOwner)))
  (bind _output_get_3 (Variables|Default|SetBombSpeed (Math|Float|Sqrt (/ (* (Math|Float|Absolute(Float) (Components|Movement|GetGravityZ (Variables|/Script/Engine.Character|GetCharacterMovement _ascharacter))) (Math|Float|Power _output_get_2 2.0)) (* (+ (* _output_get_2 (Math|Trig|Tan(Degrees) _bombdegree)) (- 0.0 (.z _output_get))) (* _returnvalue_2 _returnvalue_2 2.0)))))) ; 폭탄 초기 속력
  (Game|SpawnActorfromClass "/Game/JiSeon/BluePrints/BP_JS_Bomb.BP_JS_Bomb_C" (Transformation|GetWorldTransform (Variables|Default|GetMuzzle)) "Undefined" "MultiplyWithRoot" 0 (* _output_get_3 (Math|Trig|Sin(Degrees) _bombdegree_2) (Math|Vector|VectorUp)) (* _output_get_3 (Math|Trig|Cos(Degrees) _bombdegree_2) (Math|Vector|MakeVector (.x (Math|Vector|Normalize (- (Variables|Default|GetClick%20Location) (Transformation|GetWorldLocation (Variables|Default|GetMuzzle))))) (.y (Math|Vector|Normalize (- (Variables|Default|GetClick%20Location) (Transformation|GetWorldLocation (Variables|Default|GetMuzzle))))) 0.0)) 0))