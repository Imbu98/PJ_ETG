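; Enemy character Blueprint that exposes damage, state and team queries.
; Damaged passes the amount and dodge flag to BPDamageComponent, and GetState returns that component's current state.
; GetTeam returns a fixed enemy team value.
; MovetoPlayer and ShottoPlayer events are empty here, and the construction script only calls its parent.
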(event EventMovetoPlayer)

(event EventShottoPlayer)

(fn ConstructionScript
  (|CallParentFunction))

(fn Damaged
  (params (DamageAmount :type Float%20%28double-precision%29) (CanDodge :type Boolean))
  (Default|ComponentDamaged (Variables|Default|GetBP_DamageComponent) DamageAmount CanDodge)
  (return))

(fn GetState
  (return (Variables|/Game/HyoTaek/Compoenents/BP_DamageComponent.BP_DamageComponent_C|GetCurrentState (Variables|Default|GetBP_DamageComponent))))

(fn GetTeam
  (return (Variables|Default|GetEEnemyTeamDefinition)))