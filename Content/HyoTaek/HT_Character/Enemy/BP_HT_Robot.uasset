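; Robot enemy character that shoots at the player.
; ShottoPlayer sets the enemy AI controller's focus on the target, then spawns a team-tagged bullet at Arrow1's transform.
; MovetoPlayer is empty; blackboard-driven chase and look-at rotation logic remains in the graph but is disconnected, including the cast that supplies the focus target.
; GetState returns a fixed enum value, while construction and CheckAllDie only call the parent.
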(event EventShottoPlayer
  (bind _asbp_ht_enemy_aicontroller (Utilities|Casting|CastToBP_HT_Enemy_AIController (Pawn|GetController)))
  (AI|SetFocus _asbp_ht_enemy_aicontroller (stale _asbp_ht_player))
  (Game|SpawnActorfromClass "/Game/HyoTaek/Blueprints/Bullet/BP_HT_Bullet.BP_HT_Bullet_C" (Transformation|GetWorldTransform (Variables|Default|GetArrow1)) "Undefined" "MultiplyWithRoot" 0 "NewEnumerator1" 0))

(event EventMovetoPlayer)

(fn ConstructionScript
  (|CallParentFunction))

(fn GetState
  (return "NewEnumerator0"))

(fn CheckAllDie
  (|CallParentFunction))