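; AI controller for HT enemy characters that runs the BT_HT_EnemyAI behavior tree on possess.
; It then seeds the blackboard with AttackTarget and the pawn's IdleRange under IdealRangeKey, which it immediately overwrites with ChasingTime when the pawn is a BP_HT_EnemyChar.
; The perception update event is empty, and the logic for assigning the target and player-in-sight flag is disconnected.
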(event OnTargetPerceptionUpdated(AIPerception)
  (params (Actor :type Actor%20Object%20Reference) (Stimulus :type AI%20Stimulus%20Structure)))

(event EventBeginPlay)

(event EventPossess
  (params (PossessedPawn :type Pawn%20Object%20Reference))
  (AI|RunBehaviorTree "/Game/HyoTaek/HT_Character/Enemy/AIController/BehaviorTree/BT_HT_EnemyAI.BT_HT_EnemyAI")
  (AI|Components|Blackboard|SetValueasObject (AI|GetBlackboard 0) (Utilities|Name|MakeLiteralName "AttackTargetKey") (stale _output_get))
  (bind _idlerange (CallFunction|GetIdleRange))
  (AI|Components|Blackboard|SetValueasFloat (AI|GetBlackboard 0) (Utilities|Name|MakeLiteralName "IdealRangeKey") _idlerange)
  (bind _asbp_ht_enemy_char (Utilities|Casting|CastToBP_HT_EnemyChar (Pawn|GetControlledPawn)))
  (AI|Components|Blackboard|SetValueasFloat (AI|GetBlackboard 0) (Utilities|Name|MakeLiteralName "IdealRangeKey") (Variables|/Game/HyoTaek/HT_Character/Enemy/BP_HT_EnemyChar.BP_HT_EnemyChar_C|GetChasingTime _asbp_ht_enemy_char)))

(fn ConstructionScript)

(fn GetIdleRange
  (bind _asbp_ht_enemy_char (Utilities|Casting|CastToBP_HT_EnemyChar (Pawn|GetControlledPawn)))
  (return (Variables|/Game/HyoTaek/HT_Character/Enemy/BP_HT_EnemyChar.BP_HT_EnemyChar_C|GetIdleRange _asbp_ht_enemy_char)))