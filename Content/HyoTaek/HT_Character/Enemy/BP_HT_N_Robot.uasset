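; Ranged robot enemy that repositions and shoots at the player, driven through its AI controller's Blackboard.
; MovetoPlayer caches the target player, writes ideal range and chasing keys, then, despite its name, moves to a random reachable point around itself, clearing the chase flag on success.
; ShottoPlayer sets AI focus on the player and spawns a common bullet from an arrow component.
; GetState returns a fixed value.
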(event EventShottoPlayer
  (bind _asbp_ht_enemy_aicontroller (Utilities|Casting|CastToBP_HT_Enemy_AIController (Pawn|GetController)))
  (AI|SetFocus _asbp_ht_enemy_aicontroller (stale EventMovetoPlayer _asbp_common_player))
  (Game|SpawnActorfromClass "/Game/Common/BP_Common_Bullet.BP_Common_Bullet_C" (Transformation|GetWorldTransform (Variables|Default|GetArrow1)) "Undefined" "MultiplyWithRoot" 0 5e+02 5.0 "NewEnumerator1" 0))

(event EventMovetoPlayer
  (bind _returnvalue (AI|GetBlackboard 0))
  (bind _asbp_common_player (Utilities|Casting|CastToBP_Common_Player (AI|Components|Blackboard|GetValueasObject (AI|GetBlackboard 0) (Utilities|Name|MakeLiteralName "AttackTargetKey"))))
  (Variables|Default|SetAs%20BP%20Common%20Player _asbp_common_player)
  (AI|Components|Blackboard|SetValueasFloat _returnvalue (Utilities|Name|MakeLiteralName "IdealRangeKey") (Variables|Default|GetIdleRange))
  (AI|Components|Blackboard|SetValueasBool _returnvalue (Utilities|Name|MakeLiteralName "KeyIsChasing") true)
  (AI|AIMoveTo self (.RandomLocation (AI|Navigation|GetRandomReachablePointinRadius (Transformation|GetActorLocation) 1e+03 0 0)) 0 (Variables|Default|GetIdleRange) false
    (:OnSuccess
      (AI|Components|Blackboard|SetValueasBool _returnvalue (Utilities|Name|MakeLiteralName "KeyIsChasing") false))))

(fn ConstructionScript
  (|CallParentFunction))

(fn GetState
  (return "NewEnumerator0"))

(fn CheckAllDie
  (|CallParentFunction))