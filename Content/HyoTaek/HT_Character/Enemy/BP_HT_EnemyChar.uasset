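; Base enemy character Blueprint whose move and shoot events are empty stubs.
; Damage and state queries forward to its damage component, while the team getter reports an enemy team.
; On the die event it removes itself from its spawner's enemy array and destroys itself; if that empties the array, it first has the spawner spawn a chest and destroy the wall.
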(event EventSetStateDie
  (CallFunction|CheckAllDie))

(event EventMovetoPlayer)

(event EventShottoPlayer
  (params (FirePatternType :type E_BossFireType%20Enum :default "NewEnumerator3")))

(fn ConstructionScript
  (|CallParentFunction))

(fn CheckAllDie
  (bind _spawner (Variables|Default|GetSpawner))
  (bind _spawner_2 (Variables|Default|GetSpawner))
  (bind _enemyarray (Variables|/Game/Common/BP_CommonEnemySpawner.BP_CommonEnemySpawner_C|GetEnemyArray _spawner))
  (bind _returnvalue (Utilities|Array|RemoveItem _enemyarray self))
  (if _returnvalue
    (if (Utilities|Array|IsEmpty _enemyarray)
      (Default|SpawnChest _spawner_2)
      (Default|DestroyWall _spawner_2)
      (Actor|DestroyActor)
      (else
        (Actor|DestroyActor)))))

(fn GetBT
  (return 0))

(fn Damaged
  (params (DamageAmount :type Float%20%28double-precision%29) (CanDodge :type Boolean))
  (Default|ComponentDamaged (Variables|Default|GetBP_DamageComponent) DamageAmount CanDodge)
  (return false))

(fn GetState
  (return (Variables|/Game/HyoTaek/Compoenents/BP_DamageComponent.BP_DamageComponent_C|GetCurrentState (Variables|Default|GetBP_DamageComponent))))

(fn GetTeam
  (return (Variables|Default|GetEEnemyTeamDefinition)))