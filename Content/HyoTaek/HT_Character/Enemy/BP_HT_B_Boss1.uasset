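; Boss enemy that fires bullet-hell patterns of BP_Common_Bullet: a rotating ring, a spiral and a fan centered on its facing.
; ShottoPlayer clears the current timer and loops the selected pattern at FireRate, but only when a valid timer handle already exists.
; Tick advances the ring and spiral angles over time.
; The spiral spawns at the raw forward vector rather than the boss's location, unlike the other patterns.
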(event Custom|FirePattern3
  (bind _bulletcount (Variables|Default|GetbulletCount))
  (for _index (range 0 _bulletcount)
    (Game|SpawnActorfromClass "/Game/Common/BP_Common_Bullet.BP_Common_Bullet_C" (Math|Transform|MakeTransform (Transformation|GetActorLocation) (Math|Rotator|MakeRotator 0.0 0.0 (+ (.yaw (Transformation|GetActorRotation)) (Math|Float|Lerp (* (/ (Variables|Default|GetspreadAngle) 2.0) -1.0) (/ (Variables|Default|GetspreadAngle) 2.0) (/ _index _bulletcount)))) "1.000000,1.000000,1.000000") "Undefined" "MultiplyWithRoot" 0 2e+03 5.0 "NewEnumerator1" 0)))

(event Custom|FirePattern1
  ;[0.15 0.15 0.15 0.5] 원형
  (for _index (range 0 (Variables|Default|GetbulletCount))
    (Game|SpawnActorfromClass "/Game/Common/BP_Common_Bullet.BP_Common_Bullet_C" (Math|Transform|MakeTransform (+ (Transformation|GetActorLocation) "") (Math|Rotator|MakeRotator 0.0 0.0 (+ (* _index (/ (Math|Float|MakeLiteralFloat 3.6e+02) (Variables|Default|GetbulletCount))) (Variables|Default|GetAngleOffset))) "1.000000,1.000000,1.000000") "Undefined" "MultiplyWithRoot" 0 6e+02 5.0 "NewEnumerator1" 0)))

(event Custom|FirePattern2
  ;[0.15 0.15 0.15 0.5] 나선형
  (Game|SpawnActorfromClass "/Game/Common/BP_Common_Bullet.BP_Common_Bullet_C" (Math|Transform|MakeTransform (Transformation|GetActorForwardVector) (Math|Rotator|MakeRotator 0.0 0.0 (Variables|Default|GetcurrentAngle)) "1.000000,1.000000,1.000000") "Undefined" "MultiplyWithRoot" 0 2e+03 5.0 "NewEnumerator1" 0))

(event EventShottoPlayer
  (params (FirePatternType :type E_BossFireType%20Enum :default "NewEnumerator0"))
  (if (Utilities|Time|IsValidTimerHandle (Variables|Default|GetFirePatternHandle))
    (Utilities|Time|ClearandInvalidateTimerbyHandle (Variables|Default|GetFirePatternHandle))
    (switch Utilities|FlowControl|Switch|SwitchonE_BossFireType FirePatternType
      (:NewEnumerator0
        ;[0.15 0.15 0.15 0.5] 원형
        (bind _returnvalue (Utilities|Time|SetTimerbyEvent (delegate Custom|FirePattern1) (Variables|Default|GetFireRate) true))
        (Variables|Default|SetFirePatternHandle _returnvalue))
      (:NewEnumerator1
        ;[0.15 0.15 0.15 0.5] 나선형
        (bind _returnvalue_2 (Utilities|Time|SetTimerbyEvent (delegate Custom|FirePattern2) (Variables|Default|GetFireRate) true))
        (Variables|Default|SetFirePatternHandle _returnvalue_2))
      (:NewEnumerator2
        (bind _returnvalue_3 (Utilities|Time|SetTimerbyEvent (delegate Custom|FirePattern3) (Variables|Default|GetFireRate) true))
        (Variables|Default|SetFirePatternHandle _returnvalue_3)))))

(event EventTick
  (params (DeltaSeconds :type Float%20%28single-precision%29))
  ;[0.15 0.15 0.15 0.5] 원형 탄막
  (Variables|Default|SetAngleOffset (+ (* DeltaSeconds 15.0) (Variables|Default|GetAngleOffset)))
  ;[0.15 0.15 0.15 0.5] 나선형 탄막
  (Variables|Default|SetcurrentAngle (+ (Variables|Default|GetcurrentAngle) (* (Utilities|Time|GetWorldDeltaSeconds) (Variables|Default|GetAngleStep) 7.0))))

(fn ConstructionScript
  (|CallParentFunction))