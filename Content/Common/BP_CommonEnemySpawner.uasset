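; Room encounter spawner that spawns a boss or five weighted-random normal enemies and raises In/Out walls when the player leaves its Box.
; Only the normal branch sets IsSpawned; each enemy gets a Spawner reference back.
; Enemy type and chest rarity come from DataTable Probability×Weight running sums, re-rolling the random value on every row.
; SpawnChest and DestroyWall, not called here, provide the rarity-materialed reward and wall opening.
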(event OnComponentEndOverlap(Box)
  (params (OverlappedComponent :type Primitive%20Component%20Object%20Reference) (OtherActor :type Actor%20Object%20Reference) (OtherComp :type Primitive%20Component%20Object%20Reference) (OtherBodyIndex :type Integer))
  (bind _returnvalue (Transformation|GetActorLocation))
  (bind _randomlocation (AI|Navigation|GetRandomReachablePointinRadius _returnvalue 6e+02 0 0))
  (if (not (Variables|Default|GetIsSpawned))
    (Utilities|Casting|CastToBP_Common_Player OtherActor)
    (if (Variables|Default|GetIsBossRoom)
      (bind _returnvalue_2 (Game|SpawnActorfromClass (Utilities|Array|Get(acopy) (Variables|Default|GetBossEnemyArray)) (Math|Transform|MakeTransform (Transformation|GetWorldLocation (Variables|Default|GetSpawnAreaCenter)) "0, 0, 0" "1.000000,1.000000,1.000000") "Undefined" "MultiplyWithRoot" 0 0))
      (Utilities|Array|Add (Variables|Default|GetEnemyArray) _returnvalue_2)
      (Variables|/Game/HyoTaek/HT_Character/Enemy/BP_HT_EnemyChar.BP_HT_EnemyChar_C|SetSpawner _returnvalue_2 self)
      (CallFunction|GenerateWall)
      (else
        (for _index (range 1 (Math|Random|RandomIntegerinRange 5 5))
          (bind _returnvalue_3 (Game|SpawnActorfromClass (Utilities|Array|Get(acopy) (Variables|Default|GetnormalEnemyArray) (CallFunction|SetSpawnEnemyProbability)) (Math|Transform|MakeTransform (Math|Vector|MakeVector (.x _randomlocation) (.y _randomlocation) 0.0) "0, 0, 0" "1.000000,1.000000,1.000000") "Undefined" "MultiplyWithRoot" 0 0))
          (Utilities|Array|Add (Variables|Default|GetEnemyArray) _returnvalue_3)
          (Variables|/Game/HyoTaek/HT_Character/Enemy/BP_HT_EnemyChar.BP_HT_EnemyChar_C|SetSpawner _returnvalue_3 self)
          (CallFunction|GenerateWall))
        (Variables|Default|SetIsSpawned true)))))

(event EventBeginPlay
  (bind _outrownames (DataTable|GetDataTableRowNames "/Game/HyoTaek/Data/DataTable/DT_MonsterSpawnProbabilty.DT_MonsterSpawnProbabilty"))
  (for _array_element _outrownames
    (bind _returnvalue (Utilities|GetDataTableRow "/Game/HyoTaek/Data/DataTable/DT_MonsterSpawnProbabilty.DT_MonsterSpawnProbabilty" _array_element)
      (:then
        (Variables|Default|SetMonsterTotalProbability (+ (Variables|Default|GetMonsterTotalProbability) (* (.Probability (Utilities|Struct|BreakS_MonsterProbability _returnvalue)) (.Weight (Utilities|Struct|BreakS_MonsterProbability _returnvalue)))))))))

(fn ConstructionScript)

(fn SetChestProbability
  (params (ChestProbability :type Float%20%28double-precision%29))
  (bind _outrownames (DataTable|GetDataTableRowNames "/Game/HyoTaek/Data/DataTable/DT_ChestProbability.DT_ChestProbability"))
  (for (_array_element _array_index) _outrownames
    (bind _returnvalue (Utilities|GetDataTableRow "/Game/HyoTaek/Data/DataTable/DT_ChestProbability.DT_ChestProbability" _array_element)
      (:then
        (bind _output_get (LocalVariables|SetAcc (+ (LocalVariables|GetAcc) (* (.probability _returnvalue) (.weight _returnvalue)))))
        (if (<= (Math|Random|RandomFloatinRange 0.0 ChestProbability) _output_get)
          (return (Utilities|Enum|ByteToEnumE_Rarity (Math|Conversions|ToByte(Integer) _array_index))))))))

(fn SpawnChest
  (bind _output_get (Variables|Default|SetProbabilityDataTable (.DataTable (Utilities|Struct|BreakDataTableRowHandle (Variables|Default|GetDT_ChestProbability)))))
  (Utilities|IsValid _output_get
    (:Is%20Valid
      (Utilities|FlowControl|Sequence
        (:then_0
          (bind _outrownames (DataTable|GetDataTableRowNames (Variables|Default|GetProbabilityDataTable)))
          (for _array_element _outrownames
            (bind _returnvalue (Utilities|GetDataTableRow (Variables|Default|GetProbabilityDataTable) _array_element)
              (:then
                (bind _output_get_2 (Variables|Default|SetChestTotalProbability (+ (Variables|Default|GetChestTotalProbability) (* (.Probability (Utilities|Struct|BreakS_ChestProbability _returnvalue)) (.Weight (Utilities|Struct|BreakS_ChestProbability _returnvalue)))))))))
          (bind _rarity (CallFunction|SetChestProbability _output_get_2))
          (Variables|Default|SetChestTotalProbability 0.0))
        (:then_1
          (bind _returnvalue_2 (Game|SpawnActorfromClass "/Game/HyoTaek/Blueprints/Chest/BP_Chest.BP_Chest_C" (Math|Transform|MakeTransform (Transformation|GetWorldLocation (Variables|Default|GetSpawnAreaCenter)) "0, 0, 0" "1.000000,1.000000,1.000000") "Undefined" "MultiplyWithRoot" 0 _rarity 0))
          (Utilities|IsValid _returnvalue_2
            (:Is%20Valid
              (bind _returnvalue_3 (Utilities|GetDataTableRow "/Game/HyoTaek/Data/DataTable/DT_ChestComponent.DT_ChestComponent" (Utilities|Select :Index _rarity :NewEnumerator0 "Normal" :NewEnumerator1 "Rare" :NewEnumerator2 "Epic" :NewEnumerator3 "Legendary"))
                (:then
                  (Rendering|Material|SetMaterial (Variables|/Game/HyoTaek/Blueprints/Chest/BP_Chest.BP_Chest_C|GetStaticMesh _returnvalue_2) 0 (.chestmaterial _returnvalue_3))
                  (Collision|SetCollisionResponsetoAllChannels (Variables|Default|GetBox) "ECR_Overlap"))))))))))

(fn SetSpawnEnemyProbability
  (bind _outrownames (DataTable|GetDataTableRowNames "/Game/HyoTaek/Data/DataTable/DT_MonsterSpawnProbabilty.DT_MonsterSpawnProbabilty"))
  (for (_array_element _array_index) _outrownames
    (bind _returnvalue (Utilities|GetDataTableRow "/Game/HyoTaek/Data/DataTable/DT_MonsterSpawnProbabilty.DT_MonsterSpawnProbabilty" _array_element)
      (:then
        (bind _output_get (LocalVariables|SetAcc (+ (LocalVariables|GetAcc) (* (.probability _returnvalue) (.weight _returnvalue)))))
        (if (<= (Math|Random|RandomFloatinRange 0.0 (Variables|Default|GetMonsterTotalProbability)) _output_get)
          (return _array_index))))))

(fn DestroyWall
  (Collision|SetCollisionEnabled (Variables|Default|GetIn) "NoCollision")
  (Collision|SetCollisionEnabled (Variables|Default|GetOut) "NoCollision"))

(fn GenerateWall
  (Collision|SetCollisionProfileName (Variables|Default|GetIn) "Wall" true :!class /Script/Engine.PrimitiveComponent)
  (Collision|SetCollisionProfileName (Variables|Default|GetOut) "Wall" true :!class /Script/Engine.PrimitiveComponent))