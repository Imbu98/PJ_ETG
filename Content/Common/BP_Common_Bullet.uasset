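; BP_Common_Bullet is a team-aware projectile that moves along its forward vector each Tick at Speed, without sweeping.
; On overlap, it damages other-team BPI_Damage actors whose state is Idle, first launching any BP_HT_EnemyChar along the bullet's direction.
; After sending dodgeable damage it destroys itself unless the target's re-read state is Dodging.
; It also destroys itself on walls and other-team BP_Common_RemoveSkill actors.
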(event Collision|EventActorBeginOverlap
  (params (OtherActor :type Actor%20Object%20Reference))
  (Utilities|FlowControl|Sequence
    (:then_0
      ;[0.15 0.15 0.15 0.5] 총알 파괴 스킬
      (bind _teamdefinition (Class|BPIDamage|GetTeam(Message) OtherActor))
      (if (Utilities|Enum|NotEqual(Enum) _teamdefinition (Variables|Default|GetETeamDefinition))
        (Utilities|Casting|CastToBP_Common_RemoveSkill OtherActor)
        (Actor|DestroyActor)))
    (:then_1
      (if (Utilities|DoesObjectImplementInterface OtherActor "/Game/HyoTaek/Interface/BPI_Damage.BPI_Damage_C")
        (bind _damagestate (Class|BPIDamage|GetState(Message) OtherActor))
        (switch Utilities|FlowControl|Switch|SwitchonE_DamageState _damagestate
          (:NewEnumerator0
            (bind _teamdefinition_2 (Class|BPIDamage|GetTeam(Message) OtherActor))
            (if (Utilities|Enum|NotEqual(Enum) _teamdefinition_2 (Variables|Default|GetETeamDefinition))
              (Utilities|FlowControl|Sequence
                (:then_0
                  (bind _asbp_ht_enemy_char (Utilities|Casting|CastToBP_HT_EnemyChar OtherActor))
                  (Character|LaunchCharacter _asbp_ht_enemy_char (* (Math|Vector|Normalize (- (Transformation|GetActorForwardVector) "")) 1e+03) false false))
                (:then_1
                  ;[0.15 0.15 0.15 0.5] 현재 회피상태면 총알을 부수지 않음
                  (bind _damagestate_2 (Class|BPIDamage|GetState(Message) OtherActor))
                  (if (Utilities|Enum|Equal(Enum) _damagestate_2 "NewEnumerator2")
                    (Class|BPIDamage|Damaged(Message) OtherActor (Variables|Default|GetDamage) true)
                    (else
                      (Class|BPIDamage|Damaged(Message) OtherActor (Variables|Default|GetDamage) true)
                      (Actor|DestroyActor))))))))))
    (:then_2
      (Utilities|Casting|CastToBP_JS_Wall OtherActor)
      (Actor|DestroyActor))))

(event EventTick
  (params (DeltaSeconds :type Float%20%28single-precision%29))
  (Transformation|SetActorLocation (+ (Transformation|GetActorLocation) (* DeltaSeconds (Variables|Default|GetSpeed) (Transformation|GetActorForwardVector))) false false))

(fn ConstructionScript)