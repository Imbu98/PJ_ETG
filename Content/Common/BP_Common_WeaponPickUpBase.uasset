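; Base actor for weapon pickups that give the interacting player a gun.
; On BeginPlay it sets the Gun static mesh from the GunMesh in its pickup weapon component, if that mesh is valid.
; Interact casts to BP_Common_Player, passes the weapon, component and pickup location to the player's SpawnGun, then destroys the pickup.
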(event Collision|EventActorBeginOverlap
  (params (OtherActor :type Actor%20Object%20Reference))
  (|CallParentFunction OtherActor) ; This node is disabled and will not be called.\nDrag off pins to build functionality.
)

(event EventTick
  (params (DeltaSeconds :type Float%20%28single-precision%29))
  (|CallParentFunction DeltaSeconds) ; This node is disabled and will not be called.\nDrag off pins to build functionality.
)

(event EventInteract
  (params (Player :type Actor%20Object%20Reference))
  (bind _asbp_common_player (Utilities|Casting|CastToBP_Common_Player Player))
  (Default|SpawnGun _asbp_common_player (Variables|Default|GetWeapon) (Variables|Default|GetCPickUpWeaponComponent) (Transformation|GetActorLocation) false)
  (Actor|DestroyActor))

(event EventBeginPlay
  (bind _cpickupweaponcomponent (Variables|Default|GetCPickUpWeaponComponent))
  (Utilities|IsValid (.gunmesh _cpickupweaponcomponent)
    (:Is%20Valid
      (Components|StaticMesh|SetStaticMesh (Variables|Default|Getgun) (.gunmesh _cpickupweaponcomponent)))))

(fn ConstructionScript
  (|CallParentFunction))