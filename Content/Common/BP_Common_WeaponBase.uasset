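; Base weapon Blueprint that provides pistol, rifle and thrown-bomb fire from a Muzzle point, plus an empty shotgun stub.
; Pistol fire uses CheckAmmo to update the HUD, timed cooldown and reload, and re-equips the basic gun when limited ammo runs out.
; Rifle fire spawns bullets without checking ammo.
; Bomb fire solves projectile launch speed from gravity and a set angle to reach the cursor hit point.
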(event Custom|Reloading
  (Variables|Default|SetCanShoot true)
  (Variables|Default|SetCurrentCapacityAmmo (.ammocapacity (Variables|Default|GetCurrentWeaponComponent)))
  (Default|UpdateAmmo (Variables|Default|GetWBP%20Gun%20Bullet%20Info) (Variables|Default|GetCurrentAmmo) (.maxammo (Variables|Default|GetCurrentWeaponComponent)) (Variables|Default|GetCurrentCapacityAmmo)))

(event Custom|SetCanShoot
  (Variables|Default|SetCanShoot true))

(event EventBeginPlay
  (bind _currentweaponcomponent (Variables|Default|GetCurrentWeaponComponent))
  (|CallParentFunction)
  (Variables|Default|SetCurrentAmmo (.maxammo _currentweaponcomponent))
  (Variables|Default|SetCurrentCapacityAmmo (.ammocapacity _currentweaponcomponent))
  (bind _asbp_common_player_controller (Utilities|Casting|CastToBP_Common_PlayerController (Game|GetPlayerController 0)))
  (bind _output_get (Variables|Default|SetCommon%20Player%20Controller _asbp_common_player_controller))
  (bind _output_get_2 (Variables|Default|SetWBP%20Gun%20Bullet%20Info (Variables|/Game/Common/BP_Common_PlayerController.BP_Common_PlayerController_C|GetWBP_GunBulletInfo _output_get)))
  (Default|UpdateAmmo _output_get_2 (Variables|Default|GetCurrentAmmo) (.maxammo _currentweaponcomponent) (Variables|Default|GetCurrentCapacityAmmo)))

(event Collision|EventActorBeginOverlap
  (params (OtherActor :type Actor%20Object%20Reference))
  (|CallParentFunction OtherActor) ; This node is disabled and will not be called.\nDrag off pins to build functionality.
)

(event EventTick
  (params (DeltaSeconds :type Float%20%28single-precision%29))
  (|CallParentFunction DeltaSeconds) ; This node is disabled and will not be called.\nDrag off pins to build functionality.
)

(fn ConstructionScript
  (|CallParentFunction))

(fn PistolFire
  (if (Variables|Default|GetCanShoot)
    (if (CallFunction|CheckAmmo)
      (Utilities|Time|SetTimerbyEvent (EventDispatchers|CreateEvent :!event Custom|SetCanShoot) (.cooltime (Variables|Default|GetCurrentWeaponComponent)))
      (Game|SpawnActorfromClass "/Game/Common/BP_Common_Bullet.BP_Common_Bullet_C" (Transformation|GetWorldTransform (Variables|Default|GetMuzzle)) "Undefined" "MultiplyWithRoot" 0 "NewEnumerator0" 0)
      (Variables|Default|SetCanShoot false)
      (else
        (Variables|Default|SetCanShoot false)
        (Utilities|Time|SetTimerbyEvent (EventDispatchers|CreateEvent :!event Custom|Reloading) (Variables|Default|GetReloadTime))))))

(fn RifleFire
  (if (Variables|Default|GetCanShoot)
    (Utilities|Time|SetTimerbyEvent (EventDispatchers|CreateEvent :!event Custom|SetCanShoot) (.cooltime (Variables|Default|GetCurrentWeaponComponent)))
    (Game|SpawnActorfromClass "/Game/Common/BP_Common_Bullet.BP_Common_Bullet_C" (Transformation|GetWorldTransform (Variables|Default|GetMuzzle)) "Undefined" "MultiplyWithRoot" 0 "NewEnumerator0" 0)))

(fn BombFire
  (bind _bombdegree (Variables|Default|GetBombDegree))
  (bind _bombdegree_2 (Variables|Default|GetBombDegree))
  (bind _muzzle (Variables|Default|GetMuzzle))
  (bind _returnvalue (Transformation|GetWorldLocation _muzzle))
  (bind _returnvalue_2 (Math|Trig|Cos(Degrees) _bombdegree))
  ;[0.15 0.15 0.15 0.5] 폭탄던지기
  ;;[0.15 0.15 0.15 0.5] 클릭한 지점 위치
  (bind _output_get (Variables|Default|SetClick%20Location (.Location (Collision|BreakHitResult (.HitResult (Game|Player|GetHitResultUnderCursorbyChannel (Game|GetPlayerController 0) "TraceTypeQuery1" true))))))
  (bind _output_get_2 (Variables|Default|SetR (Math|Float|Sqrt (+ (Math|Float|Power (- (.x _output_get) (.x _returnvalue)) 2.0) (Math|Float|Power (- (.y _output_get) (.y _returnvalue)) 2.0))))) ; 시작과 도착 사이의 수평거리
  (bind _ascharacter (Utilities|Casting|CastToCharacter (Components|GetOwner)))
  (bind _output_get_3 (Variables|Default|SetBombSpeed (Math|Float|Sqrt (/ (* (Math|Float|Absolute(Float) (Components|Movement|GetGravityZ (Variables|/Script/Engine.Character|GetCharacterMovement _ascharacter))) (Math|Float|Power _output_get_2 2.0)) (* (+ (* _output_get_2 (Math|Trig|Tan(Degrees) _bombdegree)) (- 0.0 (.z _returnvalue))) (* _returnvalue_2 _returnvalue_2 2.0)))))) ; 폭탄 초기 속력
  (Game|SpawnActorfromClass "/Game/Common/BP_Common_Bomb.BP_Common_Bomb_C" (Transformation|GetWorldTransform (Variables|Default|GetMuzzle)) "Undefined" "MultiplyWithRoot" 0 (* _output_get_3 (Math|Trig|Sin(Degrees) _bombdegree_2) (Math|Vector|VectorUp)) (* _output_get_3 (Math|Trig|Cos(Degrees) _bombdegree_2) (Math|Vector|MakeVector (.x (Math|Vector|Normalize (- (Variables|Default|GetClick%20Location) (Transformation|GetWorldLocation (Variables|Default|GetMuzzle))))) (.y (Math|Vector|Normalize (- (Variables|Default|GetClick%20Location) (Transformation|GetWorldLocation (Variables|Default|GetMuzzle))))) 0.0)) "NewEnumerator0" 0))

(fn ShotgunFire)

(fn CheckAmmo
  (bind _currentweaponcomponent (Variables|Default|GetCurrentWeaponComponent))
  (bind _common_player_controller (Variables|Default|GetCommon%20Player%20Controller))
  (bind _wbp_gunbulletinfo (Variables|/Game/Common/BP_Common_PlayerController.BP_Common_PlayerController_C|GetWBP_GunBulletInfo _common_player_controller))
  (Variables|Default|SetCurrentCapacityAmmo (- (Variables|Default|GetCurrentCapacityAmmo) 1))
  (if (== (.maxammo _currentweaponcomponent) 0)
    (Default|UpdateAmmo _wbp_gunbulletinfo (Variables|Default|GetCurrentAmmo) (.maxammo _currentweaponcomponent) (Variables|Default|GetCurrentCapacityAmmo))
    (else
      (Variables|Default|SetCurrentAmmo (- (Variables|Default|GetCurrentAmmo) 1))
      (Utilities|IsValid _common_player_controller
        (:Is%20Valid
          (Utilities|IsValid _wbp_gunbulletinfo
            (:Is%20Valid
              (Default|UpdateAmmo _wbp_gunbulletinfo (Variables|Default|GetCurrentAmmo) (.maxammo (Variables|Default|GetCurrentWeaponComponent)) (Variables|Default|GetCurrentCapacityAmmo))
              (if (> (Variables|Default|GetCurrentAmmo) 0)
                _
                (else
                  (bind _asbp_ht_common_player (Utilities|Casting|CastToBP_HT_Common_Player (Components|GetOwner)))
                  (Default|EquipBasicGun _asbp_ht_common_player)
                  (return false)))))))))
  (if (> (Variables|Default|GetCurrentCapacityAmmo) 0)
    (return true)
    (else
      (return false))))