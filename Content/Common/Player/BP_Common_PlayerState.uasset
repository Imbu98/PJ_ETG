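; Player state Blueprint that tracks the player's gold and persists it through BP_SaveGame.
; On BeginPlay it loads saved gold, mirrors it to BP_GameInstance and refreshes the player's gold UI, or starts at zero without a save.
; EarnGold adds gold, updates the game instance and saves a fresh save object.
; The existence check and save use the SlotName variable, while loading hardcodes the "PlayerGold" slot.
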(event EventBeginPlay
  (bind _returnvalue (SaveGame|DoesSaveGameExist (Variables|Default|GetSlot%20Name)))
  (if _returnvalue
    (bind _returnvalue_2 (SaveGame|LoadGamefromSlot "PlayerGold"))
    (bind _asbp_save_game (Utilities|Casting|CastToBP_SaveGame _returnvalue_2))
    (Variables|Default|SetPlayerGold (Variables|/Game/Common/BP_SaveGame.BP_SaveGame_C|GetPlayerGold_Save _asbp_save_game))
    (bind _asbp_game_instance (Utilities|Casting|CastToBP_GameInstance (Game|GetGameInstance)))
    (Variables|/Game/Common/Player/BP_GameInstance.BP_GameInstance_C|SetGI_PlayerGold _asbp_game_instance (Variables|Default|GetPlayerGold))
    (bind _asbp_common_player (Utilities|Casting|CastToBP_Common_Player (Game|Player|GetPlayerPawn 0)))
    (Default|CallUpdateGoldUI _asbp_common_player)
    (else
      (Variables|Default|SetPlayerGold 0))))

(fn ConstructionScript)

(fn EarnGold
  (params (goldAmount :type Integer))
  (Variables|Default|SetPlayerGold (+ goldAmount (Variables|Default|GetPlayerGold)))
  (bind _asbp_game_instance (Utilities|Casting|CastToBP_GameInstance (Game|GetGameInstance)))
  (Variables|/Game/Common/Player/BP_GameInstance.BP_GameInstance_C|SetGI_PlayerGold _asbp_game_instance (Variables|Default|GetPlayerGold))
  (CallFunction|GameSave))

(fn GameSave
  (bind _returnvalue (SaveGame|CreateSaveGameObject "/Game/Common/BP_SaveGame.BP_SaveGame_C"))
  (bind _asbp_save_game (Utilities|Casting|CastToBP_SaveGame _returnvalue))
  (Variables|/Game/Common/BP_SaveGame.BP_SaveGame_C|SetPlayerGold_Save _asbp_save_game (Variables|Default|GetPlayerGold))
  (SaveGame|SaveGametoSlot _asbp_save_game (Variables|Default|GetSlot%20Name)))