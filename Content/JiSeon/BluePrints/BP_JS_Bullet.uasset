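; BP_JS_Bullet is a projectile actor that damages actors it overlaps and destroys walls.
; Tick moves it along its forward vector at Speed without sweeping.
; On overlap, a BPI_Damage actor reporting Idle receives dodgeable damage and the bullet destroys itself; other states receive no damage.
; An overlapped BP_JS_Wall is destroyed, with no bullet destruction in that branch.
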(event Collision|EventActorBeginOverlap
  (params (OtherActor :type Actor%20Object%20Reference))
  (Utilities|FlowControl|Sequence
    (:then_0
      (if (Utilities|DoesObjectImplementInterface OtherActor "/Game/HyoTaek/Interface/BPI_Damage.BPI_Damage_C")
        (bind _damagestate (Class|BPIDamage|GetState(Message) OtherActor))
        (switch Utilities|FlowControl|Switch|SwitchonE_DamageState _damagestate
          (:NewEnumerator0
            (Class|BPIDamage|Damaged(Message) OtherActor (Variables|Default|GetDamage) true)
            (Actor|DestroyActor)))))
    (:then_1
      (bind _asbp_js_wall (Utilities|Casting|CastToBP_JS_Wall OtherActor))
      (Actor|DestroyActor _asbp_js_wall))))

(event EventTick
  (params (DeltaSeconds :type Float%20%28single-precision%29))
  (Transformation|SetActorLocation (+ (Transformation|GetActorLocation) (* DeltaSeconds (Variables|Default|GetSpeed) (Transformation|GetActorForwardVector))) false false))

(fn ConstructionScript)