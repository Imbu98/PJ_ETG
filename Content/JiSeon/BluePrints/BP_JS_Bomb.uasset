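; BP_JS_Bomb is a bomb projectile actor that flies in a gravity arc and explodes when it overlaps a BP_JS_Wall.
; Tick moves it with a sweep using a horizontal vector plus the average of previous and current vertical velocity, smoothing frame-time variation as gravity accumulates manually.
; Wall overlap activates particles, plays an explosion sound and destroys the actor after a short delay.
; The radial damage call is unconnected, so no damage is applied.
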(event EventBeginPlay
  ;[0.15 0.15 0.15 0.5] PreviousVerticalVector 초기화
  (Variables|Default|SetPreviousVerticalVector (Variables|Default|GetVerticalVector)))

(event Collision|EventActorBeginOverlap
  (params (OtherActor :type Actor%20Object%20Reference))
  ;[0.15 0.15 0.15 0.5] 충돌시 액터 파괴
  (Utilities|Casting|CastToBP_JS_Wall OtherActor)
  (Components|Activation|Activate (Variables|Default|GetParticleSystem) false)
  (Audio|PlaySoundatLocation "/Game/StarterContent/Audio/Explosion01.Explosion01" (Transformation|GetActorLocation) "0, 0, 0" 1.0 1.0 0.0 0 0 0 0)
  (Utilities|FlowControl|Delay 0.2)
  (Actor|DestroyActor))

(event EventTick
  (params (DeltaSeconds :type Float%20%28single-precision%29))
  (bind _returnvalue (Utilities|Time|GetWorldDeltaSeconds))
  ;[0.15 0.15 0.15 0.5] 수직속도에서 중력가속도를 빼는 방식 / 델타타임에 따라 속도변화가크게달라질것을고려해이전벡터와의평균을대입
  (Transformation|SetActorLocation (+ (Transformation|GetActorLocation) (* _returnvalue (+ (Variables|Default|GetHorizontalVector) (* (+ (Variables|Default|GetPreviousVerticalVector) (Variables|Default|GetVerticalVector)) 0.5)))) true false)
  (Variables|Default|SetPreviousVerticalVector (Variables|Default|GetVerticalVector))
  (Variables|Default|SetVerticalVector (+ (Variables|Default|GetVerticalVector) (* -9.8e+02 _returnvalue (Math|Vector|VectorUp)))))

(fn ConstructionScript)